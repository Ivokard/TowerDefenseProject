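; BP_Mine is a faction-owned proximity mine that damages enemy agents who touch it.
; When a BP_Agent of another faction overlaps its Box, it spawns an explosion at the agent's location, applies fixed damage and destroys itself.
; The construction script gives the cube a dynamic material tinted with the owning faction's color.
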(event `self.Box.OnComponentBeginOverlap`
  (params (OverlappedComponent :type "PrimitiveComponent Object Reference") (OtherActor :type "Actor Object Reference") (OtherComp :type "PrimitiveComponent Object Reference") (OtherBodyIndex :type Integer) (bFromSweep :type Boolean) (SweepResult :type "HitResult Structure (by ref)"))
  (bind _asbp_agent (cast `/Game/Blueprints/BP_Agent` OtherActor))
  (if (`|EnumInequality` (`self.Faction`) (`/Game/Blueprints/BP_Agent.Faction` _asbp_agent))
    (`GameplayStatics.SpawnEmitterAtLocation` "/Game/StarterContent/Particles/P_Explosion.P_Explosion" (`self.K2_GetActorLocation` _asbp_agent))
    (`GameplayStatics.ApplyDamage` _asbp_agent 25.0)
    (`self.K2_DestroyActor`)))

(fn `UserConstructionScript`
  (bind _returnvalue (`PrimitiveComponent.CreateDynamicMaterialInstance` (`self.Cube`) 0 "/Engine/BasicShapes/BasicShapeMaterial.BasicShapeMaterial" "None"))
  (`MaterialInstanceDynamic.SetVectorParameterValue` _returnvalue "Color" (`/Game/Blueprints/BPL_Faction.GetFactionColor` (`self.Faction`))))