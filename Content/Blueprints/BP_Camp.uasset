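; BP_Camp is a faction camp actor that endlessly spawns agents for its faction.
; From BeginPlay it loops on a random delay, spawning AgentToSpawn at the Arrow1 transform, adjusted for collisions if possible, and passing on its Faction.
; The construction script tints two cube meshes with the faction color through dynamic material instances.
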(event `self.ReceiveBeginPlay`
  (`parent.ReceiveBeginPlay`)
  (`KismetSystemLibrary.Delay` (`KismetMathLibrary.RandomFloatInRange` 5.0 10.0) :!label _label)
  (`|SpawnActorFromClass` (`self.agentToSpawn`) (`SceneComponent.K2_GetComponentToWorld` (`self.Arrow1`)) "AdjustIfPossibleButAlwaysSpawn" "OverrideRootScale" null (`self.Faction`) null)
  (goto _label))

(fn `UserConstructionScript`
  (`parent.UserConstructionScript`)
  (bind _returnvalue (`PrimitiveComponent.CreateDynamicMaterialInstance` (`self.Cube1`) 0 "/Engine/BasicShapes/BasicShapeMaterial.BasicShapeMaterial" "None"))
  (`MaterialInstanceDynamic.SetVectorParameterValue` _returnvalue "Color" (`/Game/Blueprints/BPL_Faction.GetFactionColor` (`self.Faction`)))
  (bind _returnvalue_2 (`PrimitiveComponent.CreateDynamicMaterialInstance` (`self.Cube`) 0 null "None"))
  (`MaterialInstanceDynamic.SetVectorParameterValue` _returnvalue_2 "Color" (`/Game/Blueprints/BPL_Faction.GetFactionColor` (`self.Faction`))))