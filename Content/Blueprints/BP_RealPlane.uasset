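; BP_RealPlane is an AI-driven plane pawn that is tinted by its faction.
; On possession by an AI controller, it starts the BT_Plane behavior tree.
; The construction script creates a dynamic material on the Cube component and sets its Color parameter from the Faction's color.
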(event `self.ReceivePossessed`
  (params (NewController :type "Controller Object Reference"))
  (bind _asaicontroller (cast `AIController` NewController))
  (`AIController.RunBehaviorTree` _asaicontroller "/Game/AI/BT_Plane.BT_Plane"))

(fn `UserConstructionScript`
  (`parent.UserConstructionScript`)
  (bind _returnvalue (`PrimitiveComponent.CreateDynamicMaterialInstance` (`self.Cube`) 0 null "None"))
  (`MaterialInstanceDynamic.SetVectorParameterValue` _returnvalue "Color" (`/Game/Blueprints/BPL_Faction.GetFactionColor` (`self.Faction`))))