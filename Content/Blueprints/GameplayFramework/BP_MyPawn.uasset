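; BP_MyPawn is the player pawn for placing agent camps bought with money.
; Axis inputs move it forward and sideways, while BeginPlay shows the cursor, sets Game and UI input and adds the WG_InGame widget.
; Interact spawns a BP_Camp for the selected agent at the cursor's trace location if Money covers its cost, then deducts it.
; Money compounds slightly every Tick, so income depends on frame rate.
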(event `InputAxis|MoveForwardBackward`
  (params (AxisValue :type "Float (single-precision)"))
  (`self.AddMovementInput` (`self.GetActorForwardVector`) AxisValue))

(event `InputAxis|MoveLeftRight`
  (params (AxisValue :type "Float (single-precision)"))
  (`self.AddMovementInput` (`self.GetActorRightVector`) AxisValue))

(event `self.ReceiveBeginPlay`
  (bind _asplayer_controller (cast `PlayerController` (`self.GetController`)))
  (`WidgetBlueprintLibrary.SetInputMode_GameAndUIEx` _asplayer_controller null)
  (set `PlayerController.bShowMouseCursor` true _asplayer_controller)
  (bind _returnvalue (`|CreateWidget` "/Game/UI/WG_InGame.WG_InGame_C"))
  (`UserWidget.AddToViewport` _returnvalue 0))

(event `InputAction|Interact`
  (params (Key :type "Key Structure"))
  (:`Pressed`
    (if (>= (`self.money`) (`self.agentSelectedCost`))
      (`|SpawnActorFromClass` "/Game/Blueprints/BP_Camp.BP_Camp_C" (`KismetMathLibrary.Conv_VectorToTransform` (`.Location` (`GameplayStatics.BreakHitResult` (`PlayerController.GetHitResultUnderCursorByChannel` (`GameplayStatics.GetPlayerController` 0) "TraceTypeQuery1" true)))) "AdjustIfPossibleButAlwaysSpawn" "OverrideRootScale" null (`self.agentSelected`) "NewEnumerator0" null)
      (set `self.money` (- (`self.money`) (`self.agentSelectedCost`))))))

(event `self.ReceiveTick`
  (params (DeltaSeconds :type "Float (single-precision)"))
  (set `self.money` (* (`self.money`) 1.0001)))

(fn `UserConstructionScript`)